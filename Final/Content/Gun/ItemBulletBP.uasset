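; ItemBulletBP is a bullet pickup that feeds the player's inventory UI.
; On BeginPlay it caches the InventoryWB widget from the ShooterGameMode's GameUI.
; When a HeroBP with IsGun set overlaps its sphere, it hides itself and disables collision instead of being destroyed, then adds itself to the inventory's bullet list and refreshes the widget.
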(event OnComponentBeginOverlap(Sphere)
  (params (OverlappedComponent :type Primitive%20Component%20Object%20Reference) (OtherActor :type Actor%20Object%20Reference) (OtherComp :type Primitive%20Component%20Object%20Reference) (OtherBodyIndex :type Integer) (bFromSweep :type Boolean) (SweepResult :type Hit%20Result%20Structure%20%28by%20ref%29))
  (bind _inventory (Variables|Default|GetInventory))
  (bind _ashero_bp (Utilities|Casting|CastToHeroBP OtherActor))
  (if (Variables|/Game/Hero/HeroBP.HeroBP_C|GetIsGun? _ashero_bp)
    (Rendering|SetActorHiddenInGame true)
    (Collision|SetActorEnableCollision false)
    (Utilities|Array|Add (Variables|/Game/UI/InventoryWB.InventoryWB_C|GetItemBulletBP _inventory) self)
    (Default|Refresh _inventory)))

(event EventBeginPlay
  (bind _asshooter_game_mode (Utilities|Casting|CastToShooterGameMode (Game|GetGameMode)))
  (Variables|Default|SetInventory (Variables|/Game/UI/HUD.HUD_C|GetInventoryWB (Variables|/Game/ShooterGameMode.ShooterGameMode_C|GetGameUI _asshooter_game_mode))))

(fn ConstructionScript)