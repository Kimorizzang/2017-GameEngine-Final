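; Player hero Blueprint with axis-driven movement along world X/Y, axis-driven facing and a click-held punch flag.
; On BeginPlay it spawns a MousePointBP marker and shows the cursor.
; Left click sets IsPunching and moves the marker to the visibility trace hit under the cursor; release clears the flag.
; Logic to spawn and attach a gun to GunSocket exists but is disconnected and never runs.
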(event EventBeginPlay
  (bind _returnvalue (Game|SpawnActorfromClass "/Game/UI/MousePointBP.MousePointBP_C" (Math|Conversions|ToTransform(Vector) (Transformation|GetActorLocation)) "Undefined" 0 0))
  (Variables|Default|SetMouseClickPoint _returnvalue)
  (Variables|/Script/Engine.PlayerController|SetbShowMouseCursor (Game|GetPlayerController 0) true))

(event Input|ActionEvents|InputActionLeftMouseClicked
  (params (Key :type Key%20Structure :default "AnyKey"))
  (:Pressed
    (Variables|Default|SetIsPunching? true)
    (Transformation|SetActorLocation (Variables|Default|GetMouseClickPoint) (.Location (Collision|BreakHitResult (.HitResult (Game|Player|GetHitResultUnderCursorbyChannel (Game|GetPlayerController 0) "TraceTypeQuery1" true)))) false false))
  (:Released
    (Variables|Default|SetIsPunching? false)))

(event Input|AxisEvents|InputAxisMoveForward
  (params (AxisValue :type Float%20%28single-precision%29))
  (Pawn|Input|AddMovementInput "1.000000, 0, 0" AxisValue false))

(event Input|AxisEvents|InputAxisMoveRight
  (params (AxisValue :type Float%20%28single-precision%29))
  (Pawn|Input|AddMovementInput "0,1.000000, 0" AxisValue false))

(event Input|AxisEvents|InputAxisTurn
  (params (AxisValue :type Float%20%28single-precision%29))
  (if (not (Math|Float|NearlyEqual(Float) (Math|Vector|VectorLengthSquared (Math|Vector|MakeVector AxisValue (stale Input|AxisEvents|InputAxisTurnForward AxisValue) 0.0)) 0.0 0.01))
    (Transformation|SetActorRotation (Math|Conversions|RotationFromXVector (Math|Vector|MakeVector AxisValue (stale Input|AxisEvents|InputAxisTurnForward AxisValue) 0.0)))))

(event Input|AxisEvents|InputAxisTurnForward
  (params (AxisValue :type Float%20%28single-precision%29))
  (if (not (Math|Float|NearlyEqual(Float) (Math|Vector|VectorLengthSquared (Math|Vector|MakeVector (stale Input|AxisEvents|InputAxisTurn AxisValue) AxisValue 0.0)) 0.0 0.01))
    (Transformation|SetActorRotation (Math|Conversions|RotationFromXVector (Math|Vector|MakeVector (stale Input|AxisEvents|InputAxisTurn AxisValue) AxisValue 0.0)))))

(fn ConstructionScript)